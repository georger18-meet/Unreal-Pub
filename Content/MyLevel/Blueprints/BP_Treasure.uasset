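; BP_Treasure is an interactable treasure chest that the player opens and closes with the Interact action.
; A collider enables input on the actor while the player pawn overlaps it and disables it on exit.
; Interact toggles IsOpen, playing or reversing a timeline that rolls the Hinge.
; Each timeline update also sets CollectedTreasure and calls the collected-treasure event dispatcher, so it fires repeatedly during the animation.
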(event `self.TreasureBoxCollider.OnComponentBeginOverlap`
  (params (OverlappedComponent :type "PrimitiveComponent Object Reference") (OtherActor :type "Actor Object Reference") (OtherComp :type "PrimitiveComponent Object Reference") (OtherBodyIndex :type Integer) (bFromSweep :type Boolean) (SweepResult :type "HitResult Structure (by ref)"))
  ;[1 1 1] Input Management
  (if (== OtherActor (`GameplayStatics.GetPlayerPawn` 0))
    (`self.EnableInput` (`GameplayStatics.GetPlayerController` 0))))

(event `self.TreasureBoxCollider.OnComponentEndOverlap`
  (params (OverlappedComponent :type "PrimitiveComponent Object Reference") (OtherActor :type "Actor Object Reference") (OtherComp :type "PrimitiveComponent Object Reference") (OtherBodyIndex :type Integer))
  ;[1 1 1] Input Management
  (if (== OtherActor (`GameplayStatics.GetPlayerPawn` 0))
    (`self.DisableInput` (`GameplayStatics.GetPlayerController` 0))))

(event `InputAction|Interact`
  (params (Key :type "Key Structure"))
  ;[1 1 1] Interactions
  (:`Pressed`
    (if (`self.IsOpen`)
      (set `self.IsOpen` false)
      (bind (_direction _rotationx) (`Timeline|Timeline_TreasureChest` :!via `Reverse` :!label _label)
        (:`Update`
          (`SceneComponent.K2_SetRelativeRotation` (`self.Hinge`) (`KismetMathLibrary.MakeRotator` _rotationx) false false)
          (set `self.CollectedTreasure` true)
          (`self.CollectedTreasureEventDispatcher`)))
      (else
        (set `self.IsOpen` true)
        (goto _label)))))

(fn `UserConstructionScript`)