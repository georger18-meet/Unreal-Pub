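; BP_Key is a collectible key pickup that spins steadily around its yaw axis through KeyPivot on Tick.
; Its trigger box enables actor input while the player pawn overlaps it and disables input on exit.
; Pressing Interact calls CollectSpecialKey on the ThirdPersonCharacter for special keys, or sets IsCollected otherwise.
; Either path prints a message, hides the Scene hierarchy and turns off trigger collision.
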(event `self.ReceiveTick`
  (params (DeltaSeconds :type "Float (single-precision)"))
  (`SceneComponent.K2_AddLocalRotation` (`self.KeyPivot`) (`KismetMathLibrary.MakeRotator` 0.0 0.0 (* DeltaSeconds 30.0)) false false))

(event `self.KeyTriggerBox.OnComponentBeginOverlap`
  (params (OverlappedComponent :type "PrimitiveComponent Object Reference") (OtherActor :type "Actor Object Reference") (OtherComp :type "PrimitiveComponent Object Reference") (OtherBodyIndex :type Integer) (bFromSweep :type Boolean) (SweepResult :type "HitResult Structure (by ref)"))
  ;[1 1 1] Input Management
  (if (== OtherActor (`GameplayStatics.GetPlayerPawn` 0))
    (`self.EnableInput` (`GameplayStatics.GetPlayerController` 0))))

(event `self.KeyTriggerBox.OnComponentEndOverlap`
  (params (OverlappedComponent :type "PrimitiveComponent Object Reference") (OtherActor :type "Actor Object Reference") (OtherComp :type "PrimitiveComponent Object Reference") (OtherBodyIndex :type Integer))
  ;[1 1 1] Input Management
  (if (== OtherActor (`GameplayStatics.GetPlayerPawn` 0))
    (`self.DisableInput` (`GameplayStatics.GetPlayerController` 0))))

(event `InputAction|Interact`
  (params (Key :type "Key Structure"))
  ;[1 1 1] Interaction Functionality
  (:`Pressed`
    (if (`self.IsSpecial`)
      (`/Game/ThirdPersonBP/Blueprints/ThirdPersonCharacter.CollectSpecialKey` (cast `/Game/ThirdPersonBP/Blueprints/ThirdPersonCharacter` (`GameplayStatics.GetPlayerCharacter` 0) :!pure true))
      (else
        (set `self.IsCollected` true)))
    (`KismetSystemLibrary.PrintString` "Key Collected" true true (struct :`G` 1.0 :`A` 1.0))
    (`SceneComponent.SetHiddenInGame` (`self.Scene`) true true)
    (`PrimitiveComponent.SetCollisionEnabled` (`self.KeyTriggerBox`) "NoCollision")))

(fn `UserConstructionScript`)