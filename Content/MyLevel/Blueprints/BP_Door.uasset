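; BP_Door is an interactable hinged door that the player opens and closes, with optional locking.
; Its trigger box enables input while the player pawn overlaps, so Interact can toggle one of two hinge-rotation timelines, chosen by the flipped flag.
; Locked doors unlock on interaction if the linked key is collected or, when required, the character holds the special key.
; The construction script sets the initial hinge pose, forcing locked doors closed.
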(event `self.DoorBoxTrigger.OnComponentBeginOverlap`
  (params (OverlappedComponent :type "PrimitiveComponent Object Reference") (OtherActor :type "Actor Object Reference") (OtherComp :type "PrimitiveComponent Object Reference") (OtherBodyIndex :type Integer) (bFromSweep :type Boolean) (SweepResult :type "HitResult Structure (by ref)"))
  ;[1 1 1] Input Management
  (if (== OtherActor (`GameplayStatics.GetPlayerPawn` 0))
    (`self.EnableInput` (`GameplayStatics.GetPlayerController` 0))))

(event `self.DoorBoxTrigger.OnComponentEndOverlap`
  (params (OverlappedComponent :type "PrimitiveComponent Object Reference") (OtherActor :type "Actor Object Reference") (OtherComp :type "PrimitiveComponent Object Reference") (OtherBodyIndex :type Integer))
  ;[1 1 1] Input Management
  (if (== OtherActor (`GameplayStatics.GetPlayerPawn` 0))
    (`self.DisableInput` (`GameplayStatics.GetPlayerController` 0))))

(event `InputAction|Interact`
  (params (Key :type "Key Structure"))
  ;[1 1 1] Interaction Functionality
  (:`Pressed`
    (if (`self.IsInteractable`)
      (if (`self.IsLocked`)
        (if (`self.RequiresSpecialKey`)
          (if (`/Game/ThirdPersonBP/Blueprints/ThirdPersonCharacter.HasSpecialKey` (cast `/Game/ThirdPersonBP/Blueprints/ThirdPersonCharacter` (`GameplayStatics.GetPlayerCharacter` 0) :!pure true))
            (set `self.IsLocked` false :!label _label)
            (if (`self.IsFlipped`) :!label _label_2
              (if (`self.IsOpen`)
                (bind (_direction _rotation) (`Timeline|TL_DoorRotationFlipped` :!via `Reverse` :!label _label_3)
                  (:`Update`
                    (`SceneComponent.K2_SetRelativeRotation` (`self.HingePivot`) (`KismetMathLibrary.MakeRotator` 0.0 0.0 _rotation) false false))
                  (:`Finished`
                    (switch `ETimelineDirection` _direction
                      (:`Forward`
                        (set `self.IsOpen` true :!label _label_4)
                        (`KismetSystemLibrary.PrintString` "Opened Door"))
                      (:`Backward`
                        (set `self.IsOpen` false :!label _label_5)
                        (`KismetSystemLibrary.PrintString` "Closed Door")))))
                (else
                  (goto _label_3)))
              (elif (`self.IsOpen`)
                (bind (_direction_2 _rotation_2) (`Timeline|TL_DoorRotation` :!via `Reverse` :!label _label_6)
                  (:`Update`
                    (`SceneComponent.K2_SetRelativeRotation` (`self.HingePivot`) (`KismetMathLibrary.MakeRotator` 0.0 0.0 _rotation_2) false false))
                  (:`Finished`
                    (switch `ETimelineDirection` _direction_2
                      (:`Forward`
                        (goto _label_4))
                      (:`Backward`
                        (goto _label_5)))))
                (else
                  (goto _label_6))))
            (else
              (`KismetSystemLibrary.PrintString` "The Door Is Locked" true true (struct :`R` 1.0 :`B` 0.113355 :`A` 1.0) :!label _label_7)))
          (elif (`/Game/MyLevel/Blueprints/BP_Key.IsCollected` (`self.Key`))
            (goto _label)
            (else
              (goto _label_7))))
        (else
          (goto _label_2))))))

(fn `UserConstructionScript`
  (bind _hingepivot (`self.HingePivot`))
  (if (`self.IsLocked`)
    (set `self.IsOpen` false))
  (if (`self.IsOpen`)
    (if (`self.IsFlipped`)
      (`SceneComponent.K2_SetRelativeRotation` _hingepivot (struct :`Yaw` 90.0) false false)
      (else
        (`SceneComponent.K2_SetRelativeRotation` _hingepivot (struct :`Yaw` -90.0) false false)))
    (else
      (`SceneComponent.K2_SetRelativeRotation` :`self` _hingepivot))))