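; BP_ObjTalkWithNPC is a quest objective that completes once a referenced NPC has given its quest.
; On activation it runs the parent logic, then binds a handler to the NPC's given-quest event dispatcher.
; When that event fires, it checks GetIsComplete, which asks the NPC whether the quest was given, then unbinds and broadcasts OnCompleted with itself.
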(event `self.ActivateObjective`
  (`parent.ActivateObjective`)
  (add `/Game/MyLevel/Blueprints/QuestSystem/NPCs/BP_NPC.GivenQuestEventDispatcher` (`self.NPC`) (delegate `CustomEventGivenQuest`)))

(event `CustomEventGivenQuest`
  (if (`self.GetIsComplete`)
    (remove `/Game/MyLevel/Blueprints/QuestSystem/NPCs/BP_NPC.GivenQuestEventDispatcher` (`self.NPC`) (delegate `CustomEventGivenQuest`))
    (`self.OnCompleted` self)))

(fn `GetIsComplete`
  (returns (IsComplete :type Boolean))
  (return (`/Game/MyLevel/Blueprints/QuestSystem/NPCs/BP_NPC.HasGivenQuest?` (`self.NPC`))))