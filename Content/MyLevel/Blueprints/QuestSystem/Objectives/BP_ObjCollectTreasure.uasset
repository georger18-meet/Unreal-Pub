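; BP_ObjCollectTreasure is a quest objective that completes when its referenced treasure chest has been collected.
; On activation it calls the parent logic, then binds to the chest's collected-treasure event dispatcher.
; When that event fires, GetIsComplete reads the chest's CollectedTreasure value; if true, the objective unbinds and broadcasts OnCompleted with itself.
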(event `self.ActivateObjective`
  (`parent.ActivateObjective`)
  (add `/Game/MyLevel/Blueprints/BP_Treasure.CollectedTreasureEventDispatcher` (`self.TreasureChest`) (delegate `CustomEventCollecting`)))

(event `CustomEventCollecting`
  (if (`self.GetIsComplete`)
    (remove `/Game/MyLevel/Blueprints/BP_Treasure.CollectedTreasureEventDispatcher` (`self.TreasureChest`) (delegate `CustomEventCollecting`))
    (`self.OnCompleted` self)))

(fn `GetIsComplete`
  (returns (IsComplete :type Boolean))
  (return (`/Game/MyLevel/Blueprints/BP_Treasure.CollectedTreasure` (`self.TreasureChest`))))