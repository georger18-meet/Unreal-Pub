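; BP_ObjServeBeer is a quest objective that completes once the customers who want beer have been served.
; On activation it binds to the beer-check dispatcher of its Costumers.
; The first check collects those with NeedsBeer and makes them interactable.
; Every check tests NeedGotBeerCheck across that list; when all pass, it unbinds and calls OnCompleted.
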(event `self.ActivateObjective`
  (`parent.ActivateObjective`)
  (add `/Game/MyLevel/Blueprints/QuestSystem/NPCs/BP_NPC_Costumer.BeerCheckEventDispatcher` (`self.Costumers`) (delegate `CustomEvent_BeerCheck`)))

(event `CustomEvent_BeerCheck`
  (bind _costumerswantbeer (`self.CostumersWantBeer`))
  (`|ExecutionSequence`
    (:`then_0`
      (if (not (`self.Once`))
        (set `self.Once` true)
        (for _array_element (`self.Costumers`)
          (if (`/Game/MyLevel/Blueprints/QuestSystem/NPCs/BP_NPC_Costumer.NeedsBeer` _array_element)
            (`KismetArrayLibrary.Array_Add` _costumerswantbeer _array_element)
            (for _array_element_2 _costumerswantbeer
              (set `/Game/MyLevel/Blueprints/QuestSystem/NPCs/BP_NPC_Costumer.Interactable` true _array_element_2))))))
    (:`then_1`
      (set `self.AllAcountedFor` true)
      (for _array_element_3 (`self.CostumersWantBeer`)
        (bind _gotthebeer (`/Game/MyLevel/Blueprints/QuestSystem/NPCs/BP_NPC_Costumer.NeedGotBeerCheck` _array_element_3))
        (if (not _gotthebeer)
          (set `self.AllAcountedFor` false)))
      (if (`self.GetIsComplete`)
        (remove `/Game/MyLevel/Blueprints/QuestSystem/NPCs/BP_NPC_Costumer.BeerCheckEventDispatcher` (`self.Costumers`) (delegate `CustomEvent_BeerCheck`))
        (`self.OnCompleted` self)))))

(fn `GetIsComplete`
  (returns (IsComplete :type Boolean))
  (return (`self.AllAcountedFor`)))