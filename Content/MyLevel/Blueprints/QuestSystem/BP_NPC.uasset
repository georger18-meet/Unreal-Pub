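; BP_NPC is a quest-giver NPC that the player can talk to through a chat window.
; Its trigger box enables input and shows a text prompt while the player overlaps it.
; Interact toggles BPW_ChatWindow, created once with the NPC's header, quest and content text and a back-reference to the NPC.
; Tick fires the GivenQuest event dispatcher every frame while HasGivenQuest is true.
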(event `self.NPCTriggerBox.OnComponentBeginOverlap`
  (params (OverlappedComponent :type "PrimitiveComponent Object Reference") (OtherActor :type "Actor Object Reference") (OtherComp :type "PrimitiveComponent Object Reference") (OtherBodyIndex :type Integer) (bFromSweep :type Boolean) (SweepResult :type "HitResult Structure (by ref)"))
  ;[1 1 1] Input Management
  (if (== OtherActor (`GameplayStatics.GetPlayerPawn` 0))
    (`self.EnableInput` (`GameplayStatics.GetPlayerController` 0))
    (`SceneComponent.SetHiddenInGame` (`self.TextRender`) false false)))

(event `self.NPCTriggerBox.OnComponentEndOverlap`
  (params (OverlappedComponent :type "PrimitiveComponent Object Reference") (OtherActor :type "Actor Object Reference") (OtherComp :type "PrimitiveComponent Object Reference") (OtherBodyIndex :type Integer))
  ;[1 1 1] Input Management
  (if (== OtherActor (`GameplayStatics.GetPlayerPawn` 0))
    (`self.DisableInput` (`GameplayStatics.GetPlayerController` 0))
    (`SceneComponent.SetHiddenInGame` (`self.TextRender`) true false)))

(event `InputAction|Interact`
  (params (Key :type "Key Structure"))
  ;[1 1 1] Displaying Chat
  (:`Pressed`
    (if (`self.IsChatting`)
      (`KismetSystemLibrary.PrintString` "Goodbye NPC")
      (`/Game/MyLevel/Blueprints/QuestSystem/BPW_ChatWindow.CloseChatWindow` (`self.ChatWindowRef`))
      (set `self.IsChatting` false)
      (else
        (`KismetSystemLibrary.PrintString` "Hello NPC")
        (`SceneComponent.SetHiddenInGame` (`self.TextRender`) true false)
        (`/Engine/EditorBlueprintResources/StandardMacros.IsValid` (`self.ChatWindowRef`)
          (:`Is Valid`
            _)
          (:`Is Not Valid`
            (bind _returnvalue (`|CreateWidget` "/Game/MyLevel/Blueprints/QuestSystem/BPW_ChatWindow.BPW_ChatWindow_C" (`GameplayStatics.GetPlayerController` 0) (`self.NPCHeaderText`) (`self.NPCQuestText`) (`self.NPCContentText`)))
            (bind _output_get (set `self.ChatWindowRef` _returnvalue))
            (set `/Game/MyLevel/Blueprints/QuestSystem/BPW_ChatWindow.NPC_Ref` self _output_get)))
        (`UserWidget.AddToViewport` _output_get 0)
        (set `self.IsChatting` true)))))

(event `self.ReceiveTick`
  (params (DeltaSeconds :type "Float (single-precision)"))
  (if (`self.HasGivenQuest?`)
    (`self.GivenQuestEventDispatcher`)))

(fn `HasGivenQuest?`
  (returns (HasGivenQuest :type Boolean))
  (return (`self.HasGivenQuest`)))

(fn `UserConstructionScript`
  (`SceneComponent.SetHiddenInGame` (`self.TextRender`) true false))