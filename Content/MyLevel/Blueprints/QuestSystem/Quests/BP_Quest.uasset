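; BP_Quest is the base Blueprint for quests, built around a root objective collection.
; On BeginPlay it constructs and stores that root collection, populates it with objectives, then activates it.
; The construct and populate functions only print red error messages here, acting as template-method hooks for child quests to override.
; A getter exposes the root collection.
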(event `self.ReceiveBeginPlay`
  (bind _rootobjcollection (`self.ConstructRootObjectiveCollection`))
  (bind _output_get (set `self.RootObjectiveCollection` _rootobjcollection))
  (`self.PopulateObjectives` _output_get)
  (`/Game/MyLevel/Blueprints/QuestSystem/Objectives/BP_Objective.ActivateObjective` (`self.RootObjectiveCollection`)))

(fn `ConstructRootObjectiveCollection`
  (returns (RootObjCollection :type "/Game/MyLevel/Blueprints/QuestSystem/Objectives/BP_ObjCollection Object Reference"))
  (`KismetSystemLibrary.PrintString` "Error: CreateRootObjectiveCollection called for Base Class!" true true (struct :`R` 1.0 :`B` 0.005 :`A` 1.0))
  (return null))

(fn `GetRootObjectiveCollection`
  (returns (RootObjectiveCollection :type "/Game/MyLevel/Blueprints/QuestSystem/Objectives/BP_ObjCollection Object Reference"))
  (return (`self.RootObjectiveCollection`)))

(fn `PopulateObjectives`
  (params (RootObjCollection :type "/Game/MyLevel/Blueprints/QuestSystem/Objectives/BP_ObjCollection Object Reference"))
  (`KismetSystemLibrary.PrintString` "Error: PopulateObjectives called for Base Class!" true true (struct :`R` 1.0 :`B` 0.005 :`A` 1.0)))

(fn `UserConstructionScript`)