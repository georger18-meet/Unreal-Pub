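; BP_Quest_01 is a quest in the QuestSystem that takes the player through finding and talking to a bartender, finding a key and entering a side room.
; It builds a root objective collection that carries the quest's name and order-required setting.
; It then fills that collection with reach-destination and talk-to-NPC objectives, constructed at runtime and bound to destination trigger and NPC variables.
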(fn `ConstructRootObjectiveCollection`
  (returns (RootObjCollection :type "/Game/MyLevel/Blueprints/QuestSystem/Objectives/BP_ObjCollection Object Reference"))
  (bind _returnvalue (`|GenericCreateObject` "/Game/MyLevel/Blueprints/QuestSystem/Objectives/BP_ObjCollection.BP_ObjCollection_C" self (`self.OrderRequired`) (`self.ObjectiveName`)))
  (return _returnvalue))

(fn `PopulateObjectives`
  (params (RootObjCollection :type "/Game/MyLevel/Blueprints/QuestSystem/Objectives/BP_ObjCollection Object Reference"))
  (`|ExecutionSequence`
    (:`then_0`
      (bind _returnvalue (`|GenericCreateObject` "/Game/MyLevel/Blueprints/QuestSystem/Objectives/BP_ObjReachDestination.BP_ObjReachDestination_C" self (`self.DestinationTrigger0`) "Find To Bartender"))
      (`/Game/MyLevel/Blueprints/QuestSystem/Objectives/BP_ObjCollection.AddObjective` (`local.RootObjCollection`) _returnvalue))
    (:`then_1`
      (bind _returnvalue_2 (`|GenericCreateObject` "/Game/MyLevel/Blueprints/QuestSystem/Objectives/BP_ObjTalkWithNPC.BP_ObjTalkWithNPC_C" self (`self.NPC`) "Talk To Bartender"))
      (`/Game/MyLevel/Blueprints/QuestSystem/Objectives/BP_ObjCollection.AddObjective` (`local.RootObjCollection`) _returnvalue_2))
    (:`then_2`
      (bind _returnvalue_3 (`|GenericCreateObject` "/Game/MyLevel/Blueprints/QuestSystem/Objectives/BP_ObjReachDestination.BP_ObjReachDestination_C" self (`self.DestinationTrigger1`) "Find Key"))
      (`/Game/MyLevel/Blueprints/QuestSystem/Objectives/BP_ObjCollection.AddObjective` (`local.RootObjCollection`) _returnvalue_3))
    (:`then_3`
      (bind _returnvalue_4 (`|GenericCreateObject` "/Game/MyLevel/Blueprints/QuestSystem/Objectives/BP_ObjReachDestination.BP_ObjReachDestination_C" self (`self.DestinationTrigger2`) "Enter SideRoom"))
      (`/Game/MyLevel/Blueprints/QuestSystem/Objectives/BP_ObjCollection.AddObjective` (`local.RootObjCollection`) _returnvalue_4))))

(fn `UserConstructionScript`
  (`parent.UserConstructionScript`))