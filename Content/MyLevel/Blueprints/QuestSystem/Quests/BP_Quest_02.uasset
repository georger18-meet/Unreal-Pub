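; BP_Quest_02 is a treasure-hunt quest that has the player find the treasure location and then collect the treasure.
; It overrides quest construction to create a root BP_ObjCollection named after the quest, passing through its order-required setting.
; PopulateObjectives then adds a reach-destination objective bound to a destination trigger and a collect-treasure objective bound to a treasure chest.
; The event graph holds no active logic.
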(fn `ConstructRootObjectiveCollection`
  (returns (RootObjCollection :type "/Game/MyLevel/Blueprints/QuestSystem/Objectives/BP_ObjCollection Object Reference"))
  (bind _returnvalue (`|GenericCreateObject` "/Game/MyLevel/Blueprints/QuestSystem/Objectives/BP_ObjCollection.BP_ObjCollection_C" self (`self.OrderRequired`) (`self.QuestName`)))
  (return _returnvalue))

(fn `PopulateObjectives`
  (params (RootObjCollection :type "/Game/MyLevel/Blueprints/QuestSystem/Objectives/BP_ObjCollection Object Reference"))
  (`|ExecutionSequence`
    (:`then_0`
      (bind _returnvalue (`|GenericCreateObject` "/Game/MyLevel/Blueprints/QuestSystem/Objectives/BP_ObjReachDestination.BP_ObjReachDestination_C" self (`self.DestinationTrigger`) "Find The Treasure Location"))
      (`/Game/MyLevel/Blueprints/QuestSystem/Objectives/BP_ObjCollection.AddObjective` (`local.RootObjCollection`) _returnvalue))
    (:`then_1`
      (bind _returnvalue_2 (`|GenericCreateObject` "/Game/MyLevel/Blueprints/QuestSystem/Objectives/BP_ObjCollectTreasure.BP_ObjCollectTreasure_C" self (`self.TreasureChest`) "Collect The Treasure!"))
      (`/Game/MyLevel/Blueprints/QuestSystem/Objectives/BP_ObjCollection.AddObjective` (`local.RootObjCollection`) _returnvalue_2))))

(fn `UserConstructionScript`
  (`parent.UserConstructionScript`))