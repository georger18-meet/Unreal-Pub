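; BP_NPC_Costumer is a quest-system customer NPC that can be given a beer.
; If it needs beer, its BeerMug is hidden at BeginPlay.
; NPCTriggerBox enables actor input while the player pawn overlaps it and disables it on exit.
; Pressing Interact then reveals the mug and sets GotBeer, so the delivery happens only once, with no other quest notification.
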(event `self.ReceiveBeginPlay`
  (if (`self.NeedsBeer`)
    (`SceneComponent.SetVisibility` (`/Game/MyLevel/Blueprints/BP_GlassMug.Scene` (`self.BeerMug`)) false true)))

(event `self.NPCTriggerBox.OnComponentBeginOverlap`
  (params (OverlappedComponent :type "PrimitiveComponent Object Reference") (OtherActor :type "Actor Object Reference") (OtherComp :type "PrimitiveComponent Object Reference") (OtherBodyIndex :type Integer) (bFromSweep :type Boolean) (SweepResult :type "HitResult Structure (by ref)"))
  ;[1 1 1] Input Management
  (if (== OtherActor (`GameplayStatics.GetPlayerPawn` 0))
    (`self.EnableInput` (`GameplayStatics.GetPlayerController` 0))))

(event `self.NPCTriggerBox.OnComponentEndOverlap`
  (params (OverlappedComponent :type "PrimitiveComponent Object Reference") (OtherActor :type "Actor Object Reference") (OtherComp :type "PrimitiveComponent Object Reference") (OtherBodyIndex :type Integer))
  ;[1 1 1] Input Management
  (if (== OtherActor (`GameplayStatics.GetPlayerPawn` 0))
    (`self.DisableInput` (`GameplayStatics.GetPlayerController` 0))))

(event `InputAction|Interact`
  (params (Key :type "Key Structure"))
  ;[1 1 1] Interacting
  (:`Pressed`
    (if (and (not (`self.GotBeer`)) (`self.NeedsBeer`))
      (`SceneComponent.SetVisibility` (`/Game/MyLevel/Blueprints/BP_GlassMug.Scene` (`self.BeerMug`)) true true)
      (set `self.GotBeer` true))))

(fn `UserConstructionScript`)